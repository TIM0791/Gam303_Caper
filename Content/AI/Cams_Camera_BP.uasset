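; Security camera that sweeps side to side and ends the game when it spots the player.
; A looping timer runs a forward sphere trace on the Camera channel; a player hit shows failure messages, then quits the game.
; The first trace without the player starts the Timeline that yaws the Arrow at a fixed downward pitch.
; Look-at follow and timeline-stop logic exist but are never triggered here.
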(event Custom|StopTimeline
  (bind _alpha (Timeline|Timeline Stop)
    (:Update
      (Transformation|SetRelativeRotation (Variables|Default|GetArrow) (Math|Rotator|MakeRotator 0.0 -3e+01 (Math|Float|Lerp 3e+01 -3e+01 _alpha)) false false))))

(event Custom|RestartTimeline
  (bind _alpha (Timeline|Timeline Play)
    (:Update
      (Transformation|SetRelativeRotation (Variables|Default|GetArrow) (Math|Rotator|MakeRotator 0.0 -3e+01 (Math|Float|Lerp 3e+01 -3e+01 _alpha)) false false))))

(event Custom|TickTimer
  (bind _trace (Variables|Default|GetTrace))
  (bind _returnvalue (Transformation|GetWorldLocation _trace))
  (bind (_outhit _returnvalue_2) (Collision|SphereTraceByChannel _returnvalue (+ _returnvalue (* (Math|Vector|GetForwardVector _trace) 8e+02)) 1e+02 "TraceTypeQuery2" false 0 "None"))
  (if _returnvalue_2
    (if (== (.HitActor (Collision|BreakHitResult _outhit)) (Game|Player|GetPlayerPawn 0))
      (Utilities|FlowControl|DoOnce false :!label _label
        (:Completed
          (CallFunction|PlayerDetected)))
      (else
        (Utilities|FlowControl|DoOnce false :!label _label_2
          (:Completed
            (Utilities|Time|ClearandInvalidateTimerbyHandle (Variables|Default|GetFollowTimerHandle))
            (CallFunction|RestartTimeline)
            (goto _label Reset)))))
    (else
      (goto _label_2))))

(event Custom|FollowPlayer
  (bind _arrow (Variables|Default|GetArrow))
  (Transformation|SetWorldRotation _arrow (Math|Rotator|FindLookatRotation (Transformation|GetWorldLocation _arrow) (Transformation|GetActorLocation (Game|Player|GetPlayerPawn 0))) false false))

(event Custom|StartFollowTimer
  (bind _returnvalue (Utilities|Time|SetTimerbyEvent (delegate Custom|FollowPlayer) 0.05))
  (Variables|Default|SetFollowTimerHandle _returnvalue))

(event Custom|PlayerDetected
  (Development|PrintText "You have been Detected!")
  (Utilities|FlowControl|Delay 0.5)
  (Development|PrintText "BETTER LUCK NEXT TIME!")
  (Utilities|FlowControl|Delay 3.0)
  (Game|QuitGame 0 "Quit" false))

(event EventBeginPlay
  (Utilities|Time|SetTimerbyFunctionName 0 "TickTimer" 0.05 true))

(fn ConstructionScript)