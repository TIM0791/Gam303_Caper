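; AI controller that makes its pawn wander until it perceives the player, then gives chase.
; Wandering moves to random reachable nearby points, pausing briefly and repeating only after each successful move.
; AI Perception updates for the player start a fast looping timer that reissues a move toward them.
; Losing the player clears that timer and restarts wandering.
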(event OnTargetPerceptionUpdated(AIPerception)
  (params (Actor :type Actor%20Object%20Reference) (Stimulus :type AI%20Stimulus%20Structure))
  ;[0.15 0.15 0.15 0.5] Chase
  (if (== (Game|GetPlayerCharacter 0) Actor)
    (if (.bSuccessfullySensed (Utilities|Struct|BreakAIStimulus Stimulus))
      (bind _returnvalue (Utilities|Time|SetTimerbyFunctionName 0 "Chase" 0.01 true))
      (Variables|Default|SetChaseTimerHandle _returnvalue)
      (else
        (Utilities|Time|ClearandInvalidateTimerbyHandle (Variables|Default|GetChaseTimerHandle))
        (CallFunction|Wander)))))

(event Custom|Wander
  (bind _returnvalue (Pawn|GetControlledPawn))
  ;[0.15 0.15 0.15 0.5] Wander
  (AI|AIMoveTo _returnvalue (.RandomLocation (AI|Navigation|GetRandomReachablePointinRadius (Transformation|GetActorLocation _returnvalue) 8e+02 0 0)) 0 5.0 false
    (:OnSuccess
      (Utilities|FlowControl|Delay (Math|Random|RandomFloatinRange 1.0 3.0))
      (CallFunction|Wander))))

(event Custom|Chase
  ;[0.15 0.15 0.15 0.5] Chase
  (AI|AIMoveTo (Pawn|GetControlledPawn) "0, 0, 0" (Game|GetPlayerCharacter 0) 5e+01 false))

(event EventBeginPlay
  ;[0.15 0.15 0.15 0.5] Wander
  (CallFunction|Wander))

(fn ConstructionScript)