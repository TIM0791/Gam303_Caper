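; Procedural terrain that copies a static mesh into a procedural mesh and can be dented at impact points at runtime.
; On BeginPlay it reads the source's first LOD and section, calculates normals and tangents, then builds the section with collision.
; AlterMesh offsets vertices within Radius of ImpactPoint by Depth, without falloff or space conversion.
; It then updates the section in place, reusing the original normals and tangents.
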(event Custom|GenerateMesh
  (Class|ProceduralMeshComponent|CreateMeshSectionLinearColor (Variables|Default|GetProceduralMesh) 0 (Variables|Default|GetVertices) (Variables|Default|GetTriangles) (Variables|Default|GetNormals) (Variables|Default|GetUVs) 0 0 0 0 (Variables|Default|GetTangents) true false))

(event EventBeginPlay
  (Rendering|Material|SetMaterial (Variables|Default|GetProceduralMesh) 0 (Variables|Default|GetProcMaterial))
  (bind (_vertices _triangles _normals _uvs) (Class|KismetProceduralMeshLibrary|GetSectionfromStaticMesh (Variables|/Script/Engine.StaticMeshComponent|GetStaticMesh (Variables|Default|GetSourceTerrain))))
  (Variables|Default|SetVertices _vertices)
  (Variables|Default|SetTriangles _triangles)
  (Variables|Default|SetUVs _uvs)
  (bind (_normals_2 _tangents) (Class|KismetProceduralMeshLibrary|CalculateTangentsforMesh (Variables|Default|GetVertices) (Variables|Default|GetTriangles) (Variables|Default|GetUVs)))
  (Variables|Default|SetNormals _normals_2)
  (Variables|Default|SetTangents _tangents)
  (Class|ProceduralMeshComponent|UpdateMeshSectionLinearColor (Variables|Default|GetProceduralMesh) 0 (Variables|Default|GetVertices) (Variables|Default|GetNormals) (Variables|Default|GetUVs) 0 0 0 0 (Variables|Default|GetTangents) true)
  (CallFunction|GenerateMesh))

(event EventAlterMesh
  (params (ImpactPoint :type Vector :default "0, 0, 0"))
  (for (_array_element _array_index) (Variables|Default|GetVertices)
    (if (< (Math|Vector|VectorLength (- _array_element ImpactPoint)) (Variables|Default|GetRadius))
      (Utilities|Array|SetArrayElem (Variables|Default|GetVertices) _array_index (- _array_element (Variables|Default|GetDepth)))))
  (Class|ProceduralMeshComponent|UpdateMeshSectionLinearColor (Variables|Default|GetProceduralMesh) 0 (Variables|Default|GetVertices) (Variables|Default|GetNormals) (Variables|Default|GetUVs) 0 0 0 0 (Variables|Default|GetTangents) true))

(fn ConstructionScript)